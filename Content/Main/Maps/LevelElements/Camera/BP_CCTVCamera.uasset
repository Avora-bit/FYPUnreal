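; BP_CCTVCamera is a level-element security camera whose mesh pans in yaw around its placed orientation.
; On BeginPlay it caches the spawn transform, sets the bounce timeline's play rate from RotationRate and plays it.
; Each update offsets the mesh's world yaw by the timeline's Angle track scaled by RotationLimit, keeping spawn pitch and roll.
; The graph is purely rotational, with no detection or capture logic.
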(event EventBeginPlay
  (Variables|Default|SetSpawnTransform (Transformation|GetActorTransform))
  (Components|Timeline|SetPlayRate (Variables|Default|GetTimeline_Bounce) (Variables|Default|GetRotation%20Rate))
  (bind _angle (Timeline|Timeline_Bounce Play)
    (:Update
      (Transformation|SetWorldRotation (Variables|Default|GetStaticMesh) (Math|Rotator|MakeRotator (.roll (.rotation (Variables|Default|GetSpawnTransform))) (.pitch (.rotation (Variables|Default|GetSpawnTransform))) (+ (.yaw (.rotation (Variables|Default|GetSpawnTransform))) (* _angle (Variables|Default|GetRotation%20Limit)))) false false))))

(fn ConstructionScript)