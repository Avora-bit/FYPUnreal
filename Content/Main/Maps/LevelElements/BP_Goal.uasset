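; BP_Goal is a level goal actor that ends the level when the player reaches it after activation.
; It starts hidden with collision off until GoalActivated reveals it and enables collision.
; When the player overlaps GoalCol while it is active, it calls ObjectiveScore, opens the LevelCompletion level, and switches to game-and-UI input with the mouse toggled on.
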(event OnComponentBeginOverlap(GoalCol)
  (params (OverlappedComponent :type Primitive%20Component%20Object%20Reference) (OtherActor :type Actor%20Object%20Reference) (OtherComp :type Primitive%20Component%20Object%20Reference) (OtherBodyIndex :type Integer) (bFromSweep :type Boolean) (SweepResult :type Hit%20Result%20Structure%20%28by%20ref%29))
  (bind (_playerref _controllerref) (CallFunction|GetPlayerRef))
  ;[1 1 1] Open Level
  (if (== OtherActor _playerref)
    (if (Variables|Default|GetActivated)
      (Default|ObjectiveScore _playerref)
      (Game|OpenLevel(byObjectReference) "/Game/Main/UserInterface/Menus/LevelCompletion/LevelCompletion.LevelCompletion")
      (Input|SetInputModeGameandUI _controllerref 0 "DoNotLock" false true)
      (Game|SetGamePaused false)
      (Default|ToggleMouse _playerref true))))

(event Custom|GoalActivated
  ;[1 1 1] Set Activated
  (Variables|Default|SetActivated true)
  (Rendering|SetActorHiddenInGame false)
  (Collision|SetActorEnableCollision true))

(event Collision|EventActorBeginOverlap
  (params (OtherActor :type Actor%20Object%20Reference)))

(event EventTick
  (params (DeltaSeconds :type Float%20%28single-precision%29)))

(event EventBeginPlay
  ;[1 1 1] Hide On Begin Play
  (Variables|Default|SetActivated false)
  (Rendering|SetActorHiddenInGame true)
  (Collision|SetActorEnableCollision false))

(fn ConstructionScript)