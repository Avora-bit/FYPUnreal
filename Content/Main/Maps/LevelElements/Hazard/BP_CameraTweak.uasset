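; BP_CameraTweak is a level trigger volume that changes the isometric orbit camera while the IsometricOrbitCharacter is inside it.
; On BeginPlay it computes the midpoints of its own pitch and zoom ranges.
; On box overlap it copies those limits to the character, sets the midpoints as zoom and pitch targets, and forces the pitch.
; When the overlap ends it calls ResetCamera on the character.
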(event OnComponentBeginOverlap(Box)
  (params (OverlappedComponent :type Primitive%20Component%20Object%20Reference) (OtherActor :type Actor%20Object%20Reference) (OtherComp :type Primitive%20Component%20Object%20Reference) (OtherBodyIndex :type Integer) (bFromSweep :type Boolean) (SweepResult :type Hit%20Result%20Structure%20%28by%20ref%29))
  ;[1 1 1] call rollback on zoom and pitch
  (bind _asisometric_orbit_character (Utilities|Casting|CastToIsometricOrbitCharacter OtherActor))
  (Variables|/Game/Main/Player/IsometricOrbitCharacter.IsometricOrbitCharacter_C|SetPitchMin _asisometric_orbit_character (Variables|Default|GetPitchMin))
  (Variables|/Game/Main/Player/IsometricOrbitCharacter.IsometricOrbitCharacter_C|SetPitchMax _asisometric_orbit_character (Variables|Default|GetPitchMax))
  (Variables|/Game/Main/Player/IsometricOrbitCharacter.IsometricOrbitCharacter_C|SetZoomMin _asisometric_orbit_character (Variables|Default|GetZoomMin))
  (Variables|/Game/Main/Player/IsometricOrbitCharacter.IsometricOrbitCharacter_C|SetZoomMax _asisometric_orbit_character (Variables|Default|GetZoomMax))
  (Variables|/Game/Main/Player/IsometricOrbitCharacter.IsometricOrbitCharacter_C|SetZoomTarget _asisometric_orbit_character (Variables|Default|GetZoomMid))
  (bind _output_get (Variables|/Game/Main/Player/IsometricOrbitCharacter.IsometricOrbitCharacter_C|SetPitchTarget _asisometric_orbit_character (Variables|Default|GetPitchMid)))
  (Default|ForcePitch _asisometric_orbit_character _output_get))

(event OnComponentEndOverlap(Box)
  (params (OverlappedComponent :type Primitive%20Component%20Object%20Reference) (OtherActor :type Actor%20Object%20Reference) (OtherComp :type Primitive%20Component%20Object%20Reference) (OtherBodyIndex :type Integer))
  ;[1 1 1] call rollback on zoom and pitch
  (bind _asisometric_orbit_character (Utilities|Casting|CastToIsometricOrbitCharacter OtherActor))
  (Default|ResetCamera _asisometric_orbit_character))

(event EventBeginPlay
  ;[1 1 1] call rollback on zoom and pitch
  (Variables|Default|SetPitchMid (/ (+ (Variables|Default|GetPitchMin) (Variables|Default|GetPitchMax)) 2.0))
  (Variables|Default|SetZoomMid (/ (+ (Variables|Default|GetZoomMin) (Variables|Default|GetZoomMax)) 2.0)))

(fn ConstructionScript)