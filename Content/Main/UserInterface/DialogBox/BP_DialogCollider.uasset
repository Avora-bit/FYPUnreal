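; Trigger volume that shows a dialog popup when the IsometricOrbitCharacter enters its box.
; Outside tutorial mode, it appends the key bound to an input action to the text, if available.
; Entry also updates the player's dialog state and camera pitch, and plays a sound once.
; Leaving removes the popup; non-tutorial popups also expire after a delay, resetting camera and input mode and destroying the actor.
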(event OnComponentBeginOverlap(Box)
  (params (OverlappedComponent :type Primitive%20Component%20Object%20Reference) (OtherActor :type Actor%20Object%20Reference) (OtherComp :type Primitive%20Component%20Object%20Reference) (OtherBodyIndex :type Integer) (bFromSweep :type Boolean) (SweepResult :type Hit%20Result%20Structure%20%28by%20ref%29))
  (bind (_playerref _controllerref) (CallFunction|GetPlayerRef))
  (bind _title (Variables|Default|GetTitle))
  (bind _text (Variables|Default|GetText))
  (Utilities|Casting|CastToIsometricOrbitCharacter OtherActor)
  (bind _returnvalue (CallFunction|ReadInputKey (Variables|Default|GetInputActionName)))
  (if (or (Utilities|Enum|Equal(Enum) (Utilities|String|ToString(Text) _returnvalue) "None") (Variables|Default|GetIsTutorial?))
    (bind _returnvalue_2 (UserInterface|CreateWidget "/Game/Main/UserInterface/DialogBox/W_DialogPopup.W_DialogPopup_C" 0 _title _text))
    (else
      (UserInterface|CreateWidget "/Game/Main/UserInterface/DialogBox/W_DialogPopup.W_DialogPopup_C" 0 _title (Utilities|Text|ToText(String) (Utilities|String|Append (Utilities|String|ToString(Text) _text) (Utilities|String|ToString(Text) _returnvalue))))))
  (bind _output_get (Variables|Default|SetWidgetref _returnvalue_2))
  (UserInterface|Viewport|AddtoViewport _output_get 0)
  (Default|UpdateDialog (.PlayerRef (CallFunction|GetPlayerRef)) (not (Variables|Default|GetIsTutorial?)) (Variables|Default|GetPitch))
  (Utilities|FlowControl|Sequence
    (:then_0
      (Utilities|FlowControl|DoOnce false
        (:Completed
          (Audio|PlaySound2D (Variables|Default|GetSound) 1.0 1.0 0.0 0 0))))
    (:then_1
      (if (not (Variables|Default|GetIsTutorial?))
        (Utilities|FlowControl|Delay (Variables|Default|GetDuration))
        (Utilities|IsValid (Variables|Default|GetWidgetref)
          (:Is%20Valid
            (Widget|RemovefromParent (Variables|Default|GetWidgetref))
            (Variables|/Game/Main/Player/IsometricOrbitCharacter.IsometricOrbitCharacter_C|SetisDialog _playerref false)
            (Default|ResetCamera _playerref)
            (Input|SetInputModeGameandUI _controllerref 0 "DoNotLock" false true)
            (Actor|DestroyActor)))))))

(event OnComponentEndOverlap(Box)
  (params (OverlappedComponent :type Primitive%20Component%20Object%20Reference) (OtherActor :type Actor%20Object%20Reference) (OtherComp :type Primitive%20Component%20Object%20Reference) (OtherBodyIndex :type Integer))
  (bind _widgetref (Variables|Default|GetWidgetref))
  (Utilities|Casting|CastToIsometricOrbitCharacter OtherActor)
  (Utilities|IsValid _widgetref
    (:Is%20Valid
      (Widget|RemovefromParent _widgetref))))

(fn ConstructionScript)

(fn ReadInputKey
  (params (InActionName :type Name))
  (return (Class|KismetInputLibrary|KeyGetDisplayName (Utilities|Struct|BreakInputActionKeyMapping (Utilities|Array|Get(acopy) (Class|InputSettings|GetActionMappingbyName (Class|InputSettings|GetInputSettings) InActionName))) true)))