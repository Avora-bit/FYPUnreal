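; BP_Rock is a rock item that can be picked up and used through Blueprint interface events.
; Interacting plays a sound at its location and stores its item struct through StoreThisItem with a pre-allocated slot.
; Using it turns off overlap events on the sphere collider, then restores them after a timed delay.
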(event EventBPIInteract
  (Audio|SpawnSoundatLocation (Variables|Default|GetInteractSound) (Transformation|GetActorLocation) "0, 0, 0" 1.0 1.0 0.0 0 0)
  (CallFunction|StoreThisItem true (Variables|Default|GetItemStruct)))

(event EventBPIUse
  (bind _sphere_collider (Variables|Default|GetSphere%20Collider))
  (Variables|/Script/Engine.PrimitiveComponent|SetbGenerateOverlapEvents _sphere_collider false)
  (Utilities|FlowControl|Delay (Variables|Default|GetTimer))
  (Variables|/Script/Engine.PrimitiveComponent|SetbGenerateOverlapEvents _sphere_collider true))

(fn ConstructionScript)