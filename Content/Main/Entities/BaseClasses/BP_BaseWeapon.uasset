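; Base weapon Blueprint that handles firing, ammo, sound and effects for guns.
; WeaponFire runs single or delayed burst shots with looping or random gunshot audio, checks ammo unless infinite, then runs a spread line trace and spawns a projectile.
; Each shot spawns Cascade and Niagara muzzle, shell and tracer effects.
; Tick also traces with debug drawing every frame, and separate macros cover first/third-person tracers and fire montages.
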(event Custom|WeaponFire
  (bind _returnvalue (Transformation|GetActorLocation))
  (bind _cameraref (CallFunction|GetPlayerRef))
  (bind _variable (|TemporaryVariable))
  (bind _muzzlepoint (Variables|Effects|GetMuzzlePoint))
  (bind _numberofbursts (Variables|Projectile|GetNumberOfBursts))
  (bind _hitscanendlocation (Variables|DoNotTouch|GetHitscanEndLocation))
  (bind _weapontype (Variables|Projectile|GetWeaponType))
  (bind _ammoshellssocketname (Variables|Effects|GetAmmoShellsSocketName))
  (bind _emitterloc (Variables|Default|GetEmitterLoc))
  (bind _emitterloc_2 (Variables|Default|GetEmitterLoc))
  (bind _returnvalue_2 (Transformation|GetWorldLocation _emitterloc_2))
  (bind _returnvalue_3 (<= _variable _numberofbursts))
  (bind _rootcomponent (Variables|/Script/Engine.Actor|GetRootComponent _cameraref))
  (bind _returnvalue_4 (Math|Vector|GetForwardVector _rootcomponent))
  (bind _returnvalue_5 (Transformation|GetWorldLocation _rootcomponent))
  (bind _returnvalue_6 (Class|KismetMathLibrary|RandomUnitVectorinConeinRadians _returnvalue_4 0.05))
  (bind _returnvalue_7 (* _returnvalue_6 1e+04))
  (bind _returnvalue_8 (+ _returnvalue_5 _returnvalue_7))
  (bind _returnvalue_9 (Utilities|Select :Index _weapontype :Option%200 _returnvalue_8 :Option%201 _hitscanendlocation))
  (if (Variables|Projectile|GetBurstFire)
    ;[1 1 1] Burst Fire
    (Variables|DoNotTouch|SetisBurstFiring true)
    (|Assign _variable 1)
    (if _returnvalue_3 :!label _label
      (Utilities|FlowControl|Sequence
        (:then_0
          _)
        (:then_1
          (if _returnvalue_3
            (Utilities|FlowControl|Delay (Variables|Projectile|GetFireRate))
            (|Assign _variable (+ _variable 1))
            (goto _label)
            (else
              (Variables|DoNotTouch|SetisBurstFiring false :!label _label_2)))))
      (else
        (goto _label_2))))
  ;[1 1 1] Looping firing sound
  (if (Variables|Effects|GetLoopingFiringSound)
    (Utilities|FlowControl|Sequence
      (:then_0
        (if (Variables|Ammo|GetInfiniteAmmo) :!label _label_3
          (CallFunction|LinetraceWeapon :!label _label_4)
          (Game|SpawnActorfromClass (Variables|Projectile|GetProjectileToFire) (Transformation|GetWorldTransform (Variables|Default|GetEmitterLoc)) "AlwaysSpawn" "SelectDefaultAtRuntime" 0 0)
          ;[1 1 1] Muzzle Flash
          (bind _returnvalue_10 (Effects|SpawnEmitterAttached (Variables|Effects|GetMuzzleEffect) _emitterloc _muzzlepoint "0, 0, 0" "0, 0, 0" "1.000000,1.000000,1.000000" "SnapToTarget"))
          (Utilities|IsValid _returnvalue_10
            (:Is%20Valid
              (Variables|DoNotTouch|SetSpawned_MuzzleParticle _returnvalue_10))
            (:Is%20Not%20Valid
              _))
          (Niagara|SpawnSystemAttached (Variables|Effects|GetNiagara_MuzzleFlashEffect) _emitterloc _muzzlepoint "0, 0, 0" "0, 0, 0" "SnapToTarget" false)
          ;[1 1 1] Ammo shell casings FX
          (if (Variables|Effects|GetSpawnAmmoShells)
            (Effects|SpawnEmitterAttached (Variables|Effects|GetAmmoShellsParticle) _emitterloc _ammoshellssocketname "0, 0, 0" "0, 0, 0" "1.000000,1.000000,1.000000" "SnapToTarget")
            (Niagara|SpawnSystemAttached (Variables|Effects|GetNiagara_AmmoShellEffect) _emitterloc _ammoshellssocketname "0, 0, 0" "0, 0, 0" "SnapToTarget" false))
          (if (Variables|Effects|GetSpawnTracer)
            ;[1 1 1] Tracer smoke FX for TPS perspective
            (bind _returnvalue_11 (Effects|SpawnEmitteratLocation 0 _returnvalue_2))
            (Utilities|IsValid _returnvalue_11
              (:Is%20Valid
                (Effects|Components|ParticleSystem|SetVectorParameter _returnvalue_11 "ShockBeamEnd" _returnvalue_9))
              (:Is%20Not%20Valid
                _))
            (bind _returnvalue_12 (Niagara|SpawnSystematLocation 0 _returnvalue_2)) ; Set Niagara tracer here
            (Utilities|IsValid _returnvalue_12
              (:Is%20Valid
                (Effects|Components|ParticleSystem|SetVectorParameter _returnvalue_12 "ShockBeamEnd" _returnvalue_9))
              (:Is%20Not%20Valid
                _)))
          (Utilities|FlowControl|Delay 0.05) ; The only reason this Delay is here is so that the crosshair has time to spread and return to normal
          (Variables|DoNotTouch|SetIsFiring false)
          (else
            (bind _hasammo (CallFunction|AmmoCheck))
            (if _hasammo
              (Variables|DoNotTouch|SetIsFiring true)
              (goto _label_4)))))
      (:then_1
        (Utilities|FlowControl|DoOnce false
          (:Completed
            (CallFunction|LoopingFireSound true)))))
    (elif (<= (Variables|Ammo|GetAmmoCurrent) 0)
      (goto _label_3)
      (else
        (switch int (Math|Random|RandomInteger 3)
          (:Default
            _)
          (:0
            (Audio|SpawnSoundatLocation "/Game/Main/SoundEffects/NewSoundStuffs/Gunshot_1.Gunshot_1" _returnvalue "0, 0, 0" 1.0 1.0 0.0 0 0)
            (goto _label_3))
          (:1
            (Audio|SpawnSoundatLocation "/Game/Main/SoundEffects/NewSoundStuffs/Gunshot_2.Gunshot_2" _returnvalue "0, 0, 0" 1.0 1.0 0.0 0 0)
            (goto _label_3))
          (:2
            _))
        (Audio|SpawnSoundatLocation "/Game/Main/SoundEffects/NewSoundStuffs/Gunshot_3.Gunshot_3" _returnvalue "0, 0, 0" 1.0 1.0 0.0 0 0)
        (goto _label_3)))))

(event Custom|Reset%20Weapon%20Params
  (Variables|DoNotTouch|SetIsFiring false)
  (Variables|DoNotTouch|SetisBurstFiring false))

(event Custom|ResetLoopSound
  ;[1 1 1] Looping firing sound
  (Utilities|FlowControl|DoOnce false) ; enters at Reset
)

(event EventTick
  (params (DeltaSeconds :type Float%20%28single-precision%29))
  (bind _emitterloc (Variables|Default|GetEmitterLoc))
  (bind _returnvalue (Transformation|GetWorldLocation _emitterloc))
  (CallFunction|LineTraceWeapon)
  (Collision|LineTraceByChannel _returnvalue (+ _returnvalue (* (Math|Vector|GetForwardVector _emitterloc) 1e+03)) "TraceTypeQuery1" false 0 "ForOneFrame"))

(fn ConstructionScript)

(fn AmmoCheck
  (Math|Integer|CompareInt (Variables|Ammo|GetAmmoCurrent)
    (:>
      (Variables|Ammo|SetAmmoCurrent (- (Variables|Ammo|GetAmmoCurrent) 1))
      (return true))
    (:==
      _)
    (:<
      _))
  (Variables|Ammo|SetAmmoCurrent 0)
  (return false))

(fn LineTraceWeapon
  (bind _bulletspread (Variables|Projectile|GetBulletSpread))
  (bind _emitterloc (Variables|Default|GetEmitterLoc))
  (bind _returnvalue (Transformation|GetWorldLocation _emitterloc))
  (bind _returnvalue_2 (Math|Vector|GetForwardVector _emitterloc))
  (bind _returnvalue_3 (* _returnvalue_2 1e+03))
  (bind _returnvalue_4 (+ _returnvalue _returnvalue_3))
  (bind (_x _y _z) (Math|Vector|BreakVector _returnvalue_4))
  (bind (_outhit _returnvalue_5) (Collision|LineTraceByChannel _returnvalue (Math|Vector|MakeVector (+ _x (Math|Random|RandomFloatinRange (* _bulletspread -1.0) _bulletspread)) (+ _y (Math|Random|RandomFloatinRange (* _bulletspread -1.0) _bulletspread)) (+ _z (Math|Random|RandomFloatinRange (* _bulletspread -1.0) _bulletspread))) "TraceTypeQuery1" false 0 "ForOneFrame"))
  (return _outhit _returnvalue_5))

(fn LoopingFireSound
  (params (Starting :type Boolean))
  (if Starting
    (if (> (Variables|Ammo|GetAmmoCurrent) 0)
      (bind _returnvalue (Audio|SpawnSoundAttached (Variables|Effects|GetFiringSound_Looping) 0 "None" "0, 0, 0" "0, 0, 0" "KeepRelativeOffset" false 1.0 1.0 0.0 0 0))
      (Variables|DoNotTouch|SetSpawnedLoopFireSound _returnvalue))))