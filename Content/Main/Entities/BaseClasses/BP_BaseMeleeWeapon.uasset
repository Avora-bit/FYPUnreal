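; Base melee weapon Blueprint that turns both the primary fire and ADS inputs into the same knife-style swing.
; Each swing plays one of two random montages on the player's mesh and a random swing sound, with a flag blocking overlapping attacks.
; After a delay timed to impact, a short debug-drawn Visibility line trace from EmitterLoc applies point damage to the hit actor, then the flag clears.
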(event Custom|ADS_Override
  (bind _returnvalue (Transformation|GetActorLocation))
  (bind _emitterloc (Variables|Default|GetEmitterLoc))
  (bind _returnvalue_2 (Transformation|GetWorldLocation _emitterloc))
  (if (not (Variables|Default|GetisMeleeAttacking))
    (Variables|Default|SetisMeleeAttacking true)
    (Animation|Montage|MontagePlay (Components|SkeletalMesh|GetAnimInstance (Variables|/Script/Engine.Character|GetMesh (.PlayerRef (CallFunction|GetPlayerRef)))) (select (Math|Random|RandomBool) (Variables|Default|GetMeleeMontage2) (Variables|Default|GetMeleeMontage1)) (Variables|Default|GetMontagePlayRateSpeed) "Duration" 0.0 true)
    (switch int (Math|Random|RandomInteger 3)
      (:Default
        (Audio|SpawnSoundatLocation "/Game/Main/SoundEffects/NewSoundStuffs/Knife_Swing_3.Knife_Swing_3" _returnvalue "0, 0, 0" 1.0 1.0 0.0 0 0 :!label _label))
      (:0
        (Audio|SpawnSoundatLocation "/Game/Main/SoundEffects/NewSoundStuffs/Knife_Swing_1.Knife_Swing_1" _returnvalue "0, 0, 0" 1.0 1.0 0.0 0 0))
      (:1
        (Audio|SpawnSoundatLocation "/Game/Main/SoundEffects/NewSoundStuffs/Knife_Swing_2.Knife_Swing_2" _returnvalue "0, 0, 0" 1.0 1.0 0.0 0 0))
      (:2
        (goto _label)))
    (Utilities|FlowControl|Delay (Variables|Default|GetDelayUntilImpact))
    (bind (_outhit _returnvalue_3) (Collision|LineTraceByChannel _returnvalue_2 (+ _returnvalue_2 (* (Math|Vector|GetForwardVector _emitterloc) 1e+02)) "TraceTypeQuery1" false (Variables|Default|GetActorsToIgnore) "ForDuration"))
    (if _returnvalue_3
      (Game|Damage|ApplyPointDamage (.HitActor (Collision|BreakHitResult _outhit)) (Variables|Default|GetDamage) (.Location (Collision|BreakHitResult _outhit)) _outhit 0 self))
    (Variables|Default|SetisMeleeAttacking false)))

(event Custom|WeaponFire_1
  (bind _returnvalue (Transformation|GetActorLocation))
  (bind _emitterloc (Variables|Default|GetEmitterLoc))
  (bind _returnvalue_2 (Transformation|GetWorldLocation _emitterloc))
  (if (not (Variables|Default|GetisMeleeAttacking))
    (Variables|Default|SetisMeleeAttacking true)
    (Animation|Montage|MontagePlay (Components|SkeletalMesh|GetAnimInstance (Variables|/Script/Engine.Character|GetMesh (.PlayerRef (CallFunction|GetPlayerRef)))) (select (Math|Random|RandomBool) (Variables|Default|GetMeleeMontage2) (Variables|Default|GetMeleeMontage1)) (Variables|Default|GetMontagePlayRateSpeed) "Duration" 0.0 true)
    (switch int (Math|Random|RandomInteger 3)
      (:Default
        (Audio|SpawnSoundatLocation "/Game/Main/SoundEffects/NewSoundStuffs/Knife_Swing_3.Knife_Swing_3" _returnvalue "0, 0, 0" 1.0 1.0 0.0 0 0 :!label _label))
      (:0
        (Audio|SpawnSoundatLocation "/Game/Main/SoundEffects/NewSoundStuffs/Knife_Swing_1.Knife_Swing_1" _returnvalue "0, 0, 0" 1.0 1.0 0.0 0 0))
      (:1
        (Audio|SpawnSoundatLocation "/Game/Main/SoundEffects/NewSoundStuffs/Knife_Swing_2.Knife_Swing_2" _returnvalue "0, 0, 0" 1.0 1.0 0.0 0 0))
      (:2
        (goto _label)))
    (Utilities|FlowControl|Delay (Variables|Default|GetDelayUntilImpact))
    (bind (_outhit _returnvalue_3) (Collision|LineTraceByChannel _returnvalue_2 (+ _returnvalue_2 (* (Math|Vector|GetForwardVector _emitterloc) 1e+02)) "TraceTypeQuery1" false (Variables|Default|GetActorsToIgnore) "ForDuration"))
    (if _returnvalue_3
      (Game|Damage|ApplyPointDamage (.HitActor (Collision|BreakHitResult _outhit)) (Variables|Default|GetDamage) (.Location (Collision|BreakHitResult _outhit)) _outhit 0 self))
    (Variables|Default|SetisMeleeAttacking false)))

(fn ConstructionScript)