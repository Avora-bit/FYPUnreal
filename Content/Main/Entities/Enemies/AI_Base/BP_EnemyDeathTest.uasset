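; BP_EnemyDeathTest is an enemy character testing death behavior, with a radial health widget that yaws to face the player camera.
; Damage reduces clamped health and updates the widget.
; At zero health, a timeline repeatedly enables mesh physics with a downward impulse.
; While the enemy overlaps BP_SunRays, that timeline also swaps in M_SOL and animates the material and NSLeak Niagara effect.
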(event EventTick
  (params (DeltaSeconds :type Float%20%28single-precision%29))
  (Transformation|SetWorldRotation (Variables|Default|GetRadialHealth) (Math|Rotator|MakeRotator 0.0 9e+01 (- (.yaw (Transformation|GetWorldRotation (Variables|/Game/Main/Player/IsometricOrbitCharacter.IsometricOrbitCharacter_C|GetCamera (stale EventBeginPlay _output_get)))) 1.8e+02)) false false))

(event EventBeginPlay
  (Utilities|FlowControl|Sequence
    (:then_0
      (bind _asisometric_orbit_character (Utilities|Casting|CastToIsometricOrbitCharacter (Game|GetPlayerCharacter 0)))
      (bind _output_get (Variables|Default|SetCharacter%20Reference _asisometric_orbit_character)))
    (:then_1
      (bind _asw_radial_health (Utilities|Casting|CastToW_RadialHealth (UserInterface|GetWidget (Variables|Default|GetRadialHealth))))
      (Variables|/Game/Main/UserInterface/Health/W_RadialHealth.W_RadialHealth_C|SetHealth _asw_radial_health (Variables|Default|GetHealth))
      (Variables|/Game/Main/UserInterface/Health/W_RadialHealth.W_RadialHealth_C|SetMaxHealth _asw_radial_health (Variables|Default|GetMaxHealth)))))

(event Game|Damage|EventAnyDamage
  (params (Damage :type Float%20%28single-precision%29) (DamageType :type Damage%20Type%20Object%20Reference) (InstigatedBy :type Controller%20Object%20Reference) (DamageCauser :type Actor%20Object%20Reference))
  (bind _mesh (Variables|Character|GetMesh))
  (Variables|Default|SetHealth (Math|Float|Clamp(Float) (- (Variables|Default|GetHealth) Damage) 0.0 (Variables|Default|GetMaxHealth)))
  (bind _asw_radial_health (Utilities|Casting|CastToW_RadialHealth (UserInterface|GetWidget (Variables|Default|GetRadialHealth))))
  (bind _output_get (Variables|/Game/Main/UserInterface/Health/W_RadialHealth.W_RadialHealth_C|SetHealth _asw_radial_health (Variables|Default|GetHealth)))
  (Variables|/Game/Main/UserInterface/Health/W_RadialHealth.W_RadialHealth_C|SetMaxHealth _asw_radial_health (Variables|Default|GetMaxHealth))
  (Math|Float|CompareFloat _output_get 0.0
    (:==
      (bind _tl_animation (Timeline|Timeline Play)
        (:Update
          (if (Utilities|Array|IsNotEmpty (Collision|GetOverlappingActors "/Game/Main/Maps/LevelElements/BP_SunRays.BP_SunRays_C" :!class /Script/Engine.Actor))
            (Niagara|SetNiagaraVariable(Float) (Variables|Default|GetNS_Leak) "User_Animation" _tl_animation)
            (Rendering|Material|SetMaterial (Variables|Character|GetMesh) 0 "/Game/DissolveTesting/M_SOL.M_SOL")
            (Rendering|Material|SetScalarParameterValueonMaterials (Variables|Character|GetMesh) "Animation" _tl_animation)
            (Utilities|FlowControl|Sequence
              (:then_0
                _)))
          (Physics|SetSimulatePhysics _mesh true)
          (Physics|AddImpulse _mesh "0.000000,0.000000,-600.000000" "None" false))))
    (:<
      (Timeline|Timeline PlayFromStart))))

(fn ConstructionScript)

(fn UpdateWalkSpeed
  (params (NewWalkSpeed :type Float%20%28double-precision%29))
  (Variables|/Script/Engine.CharacterMovementComponent|SetMaxWalkSpeed (Variables|Character|GetCharacterMovement) NewWalkSpeed))