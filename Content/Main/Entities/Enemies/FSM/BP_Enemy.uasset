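; Base enemy character with an enum-driven state machine, sun damage-over-time and a camera-facing radial health bar.
; Tick drives idle patrol between random waypoints, skipping recent ones; state changes switch walk/run speed.
; An overlap sphere gates bone-targeted sight traces, but their hits are unused and other patrol modes are disconnected.
; Zero health triggers ragdoll and Death; corpses touching BP_SunRays play a material/Niagara animation, then are destroyed.
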(event OnComponentBeginOverlap(DetectionSphere)
  (params (OverlappedComponent :type Primitive%20Component%20Object%20Reference) (OtherActor :type Actor%20Object%20Reference) (OtherComp :type Primitive%20Component%20Object%20Reference) (OtherBodyIndex :type Integer) (bFromSweep :type Boolean) (SweepResult :type Hit%20Result%20Structure%20%28by%20ref%29))
  ;[1 1 1] Player Detection
  (Utilities|Casting|CastToIsometricOrbitCharacter OtherActor)
  (Variables|AI|SetPlayerInRange true))

(event OnComponentEndOverlap(DetectionSphere)
  (params (OverlappedComponent :type Primitive%20Component%20Object%20Reference) (OtherActor :type Actor%20Object%20Reference) (OtherComp :type Primitive%20Component%20Object%20Reference) (OtherBodyIndex :type Integer))
  ;[1 1 1] Player Detection
  (Utilities|Casting|CastToIsometricOrbitCharacter OtherActor)
  (Variables|AI|SetPlayerInRange false))

(event Custom|Start%20DOT
  ;[1 1 1] Damage from Sun - DOT, constant
  (bind _returnvalue (Utilities|Time|SetTimerbyEvent (delegate Custom|Take%20DOT) (Variables|Combat|GetDOT%20Rate) true))
  (Variables|Combat|SetDOT%20Tick _returnvalue))

(event Custom|End%20DOT
  ;[1 1 1] Damage from Sun - DOT, constant
  (Utilities|Time|ClearandInvalidateTimerbyHandle (Variables|Combat|GetDOT%20Tick)))

(event Custom|Take%20DOT
  ;[1 1 1] Damage from Sun - DOT, constant
  (Game|Damage|ApplyDamage self (Variables|Default|GetDot%20Damage) 0 0))

(event Custom|OnStateChange
  (params (Prev%20State :type E_AIState%20Enum :default "NewEnumerator0") (Next%20State :type E_AIState%20Enum :default "NewEnumerator0"))
  (bind _output_get (Variables|AI|SetAIState Next%20State))
  (switch Utilities|FlowControl|Switch|SwitchonE_AIState _output_get
    (:NewEnumerator0
      (CallFunction|ChangeSpeedWalk :!label _label))
    (:NewEnumerator2
      (goto _label))
    (:NewEnumerator3
      (CallFunction|ChangeSpeedRun :!label _label_2))
    (:NewEnumerator4
      (goto _label_2))
    (:NewEnumerator5
      (goto _label_2))))

(event EventBeginPlay
  (Utilities|FlowControl|Sequence
    (:then_0
      (Variables|AI|SetAIControllerRef (AI|GetAIController self))
      (Variables|AI|SetPlayerRef (Game|GetPlayerCharacter 0)))
    (:then_1
      (bind _asw_radial_health (Utilities|Casting|CastToW_RadialHealth (UserInterface|GetWidget (Variables|Default|GetRadialHealth))))
      (Variables|/Game/Main/UserInterface/Health/W_RadialHealth.W_RadialHealth_C|SetHealth _asw_radial_health (Variables|Combat|GetHealth))
      (Variables|/Game/Main/UserInterface/Health/W_RadialHealth.W_RadialHealth_C|SetMaxHealth _asw_radial_health (Variables|Combat|GetMaxHealth)))
    (:then_2
      (Utilities|Array|Add (Variables|Movement|GetIndexLastVisited) (Variables|Movement|GetWaypointIndex)))))

(event EventTick
  (params (DeltaSeconds :type Float%20%28single-precision%29))
  (bind _waypointarray (Variables|Movement|GetWaypointArray))
  (bind _randomchangewaittime (Variables|Movement|GetRandomChangeWaitTime))
  (bind _indexarray (Variables|Movement|GetIndexArray))
  (bind _mesh (Variables|Character|GetMesh))
  (bind _indexlastvisited (Variables|Movement|GetIndexLastVisited))
  (Utilities|FlowControl|Sequence
    (:then_0
      (Utilities|FlowControl|Delay (Variables|AI|GetAITick))
      ;[1 1 1] detection here
      (if (Variables|AI|GetPlayerInRange)
        (CallFunction|CastRaysatPlayer))
      (switch Utilities|FlowControl|Switch|SwitchonE_AIState (Variables|AI|GetAIState)
        (:NewEnumerator0
          (CallFunction|AwarenessReduction)
          ;[1 1 1] Has 4 idle states, selected during editor placement
          ;;[1 1 1] Random patrol, entity moves to random allocated point not visited recently
          (if (Variables|Movement|GetCanMovetoNext)
            (Variables|Movement|SetCanMovetoNext false)
            (Utilities|Array|Clear _indexarray)
            (for (_ _array_index) _waypointarray
              (Utilities|Array|Add _indexarray _array_index))
            (for _array_element (Variables|Movement|GetIndexLastVisited)
              (Utilities|Array|RemoveItem _indexarray _array_element))
            (bind _output_get (Variables|Movement|SetWaypointIndex (.OutItem (Utilities|Array|Random _indexarray))))
            (bind _returnvalue (Utilities|Array|Add _indexlastvisited _output_get))
            (Math|Integer|CompareInt _returnvalue (Variables|Movement|GetLastIndexCount)
              (:>
                (Utilities|Array|RemoveIndex _indexlastvisited :!label _label))
              (:==
                (goto _label))
              (:<
                _))
            (bind _asynctaskproxy (AI|AIMoveTo (Variables|AI|GetAIControllerRef) "0, 0, 0" (Utilities|Array|Get(acopy) _waypointarray _output_get) -1.0 "Default" "Default" true false)
              (:then
                (Variables|Movement|SetAIMoveToRef _asynctaskproxy))
              (:OnRequestFailed
                (Utilities|FlowControl|Delay (+ (Variables|Movement|GetBaseWaitTime) (Math|Random|RandomFloatinRange (* _randomchangewaittime -1.0) _randomchangewaittime)) :!label _label_2)
                (Variables|Movement|SetCanMovetoNext true))
              (:OnMoveFinished
                (goto _label_2)))))
        (:NewEnumerator5)))
    (:then_1
      (if (and (Utilities|Enum|Equal(Enum) (Variables|AI|GetAIState) "NewEnumerator6") (Utilities|Array|IsNotEmpty (Collision|GetOverlappingActors "/Game/Main/Maps/LevelElements/Hazard/BP_SunRays.BP_SunRays_C" :!class /Script/Engine.Actor)))
        (bind _tl_animation (Timeline|Timeline_0 Play)
          (:Update
            (Niagara|SetNiagaraVariable(Float) (Variables|Default|GetNS_Leak) "User_Animation" _tl_animation)
            (Rendering|Material|SetMaterial _mesh 0 "/Game/Main/Entities/Enemies/DissolveBurnVFX/M_SOL.M_SOL")
            (Rendering|Material|SetMaterial _mesh 1 "/Game/Main/Entities/Enemies/DissolveBurnVFX/M_SOL.M_SOL")
            (Rendering|Material|SetScalarParameterValueonMaterials _mesh "Animation" _tl_animation))
          (:Finished
            (Actor|DestroyActor)))
        (else
          (Timeline|Timeline_0 Stop))))
    (:then_2
      (Transformation|SetWorldRotation (Variables|Default|GetRadialHealth) (Math|Rotator|MakeRotator 0.0 9e+01 (- (.yaw (Transformation|GetWorldRotation (Variables|/Script/Engine.Actor|GetRootComponent (Game|GetPlayerCameraManager 0)))) 1.8e+02)) false false))))

(event Game|Damage|EventAnyDamage
  (params (Damage :type Float%20%28single-precision%29) (DamageType :type Damage%20Type%20Object%20Reference) (InstigatedBy :type Controller%20Object%20Reference) (DamageCauser :type Actor%20Object%20Reference))
  (Variables|Combat|SetHealth (Math|Float|Clamp(Float) (- (Variables|Combat|GetHealth) Damage) 0.0 (Variables|Combat|GetMaxHealth)))
  (bind _asw_radial_health (Utilities|Casting|CastToW_RadialHealth (UserInterface|GetWidget (Variables|Default|GetRadialHealth))))
  (bind _output_get (Variables|/Game/Main/UserInterface/Health/W_RadialHealth.W_RadialHealth_C|SetHealth _asw_radial_health (Variables|Combat|GetHealth)))
  (Variables|/Game/Main/UserInterface/Health/W_RadialHealth.W_RadialHealth_C|SetMaxHealth _asw_radial_health (Variables|Combat|GetMaxHealth))
  (Math|Float|CompareFloat _output_get 0.0
    (:==
      _)
    (:<
      _))
  (Physics|SetSimulatePhysics (Variables|Character|GetMesh) true)
  (Collision|SetCollisionEnabled (Variables|Collision|GetCapsuleComponent) "NoCollision")
  (CallFunction|UpdateHighlight false)
  (CallFunction|OnStateChange (Variables|AI|GetAIState) "NewEnumerator6"))

(fn ConstructionScript)

(fn AwarenessReduction
  (Variables|AI|SetCurrMeter (Math|Float|Clamp(Float) (- (Variables|AI|GetCurrMeter) (Variables|AI|GetMeterTick)) 0.0 (Variables|AI|GetMaxMeter))))

(fn AwarenessChange
  (params (Value :type Float%20%28double-precision%29))
  (Variables|AI|SetCurrMeter (Math|Float|Clamp(Float) (+ (Variables|AI|GetCurrMeter) Value) 0.0 (Variables|AI|GetMaxMeter))))

(fn UpdateHighlight
  (params (HighlightState :type Boolean)))

(fn ChangeSpeedWalk
  (Variables|/Script/Engine.CharacterMovementComponent|SetMaxWalkSpeed (Variables|Character|GetCharacterMovement) (Variables|Movement|GetWalkSpeed)))

(fn ChangeSpeedRun
  (Variables|/Script/Engine.CharacterMovementComponent|SetMaxWalkSpeed (Variables|Character|GetCharacterMovement) (Variables|Movement|GetRunSpeed)))

(fn CastRaysatPlayer
  (Variables|AI|SetNumPlayerBones 0)
  (bind _asisometric_orbit_character (Utilities|Casting|CastToIsometricOrbitCharacter (Variables|AI|GetPlayerRef)))
  (bind (_head _pelvis _left_hand _right_hand _left_shoulder _right_shoulder _left_foot _right_foot) (Default|GetAllBoneLocation _asisometric_orbit_character))
  (Utilities|FlowControl|Sequence
    (:then_0
      ;[1 1 1] Head, Pelvis
      (Collision|LineTraceByChannel (Transformation|GetWorldLocation (Variables|Default|GetHead)) _head "TraceTypeQuery1" false 0 "ForOneFrame"))
    (:then_1
      ;[1 1 1] Hands
      (Collision|LineTraceByChannel (Transformation|GetWorldLocation (Variables|Default|GetHead)) _left_hand "TraceTypeQuery1" false 0 "ForOneFrame"))
    (:then_2
      (if (Variables|/Script/Engine.Character|GetbIsCrouched _asisometric_orbit_character)
        (return (Variables|AI|GetCanSeePlayer) (Variables|AI|GetCenterMass))
        (else
          (Utilities|FlowControl|Sequence
            (:then_0
              ;[1 1 1] Shoulders
              (Collision|LineTraceByChannel (Transformation|GetWorldLocation (Variables|Default|GetHead)) _left_shoulder "TraceTypeQuery1" false 0 "ForOneFrame"))
            (:then_1
              ;[1 1 1] Feet
              (Collision|LineTraceByChannel (Transformation|GetWorldLocation (Variables|Default|GetHead)) _left_foot "TraceTypeQuery1" false 0 "ForOneFrame"))
            (:then_2
              (return (Variables|AI|GetCanSeePlayer) (Variables|AI|GetCenterMass)))))))))

(fn EnemyRef
  (return 0))