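; Base enemy character with a radial health widget turned to the camera's yaw, walk-speed and highlight helpers, and a timer-driven sun damage-over-time.
; Damage updates the widget; at zero health the enemy ragdolls with a downward impulse, losing capsule collision and highlight.
; While a dead enemy overlaps BP_SunRays, a timeline drives an M_SOL material and Niagara animation, destroying the actor when finished.
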(event Custom|Start%20DOT
  ;[1 1 1] Sun Damage OT
  (bind _returnvalue (Utilities|Time|SetTimerbyEvent (delegate Custom|Take%20DOT) (Variables|Default|GetDot%20Rate) true))
  (Variables|Default|SetDot%20Tick _returnvalue))

(event Custom|End%20DOT
  ;[1 1 1] Sun Damage OT
  (Utilities|Time|ClearandInvalidateTimerbyHandle (Variables|Default|GetDot%20Tick)))

(event Custom|Take%20DOT
  ;[1 1 1] Sun Damage OT
  (Game|Damage|ApplyDamage self (Variables|Default|GetDot%20Damage) 0 0))

(event Game|Damage|EventAnyDamage
  (params (Damage :type Float%20%28single-precision%29) (DamageType :type Damage%20Type%20Object%20Reference) (InstigatedBy :type Controller%20Object%20Reference) (DamageCauser :type Actor%20Object%20Reference))
  (bind _mesh (Variables|Character|GetMesh))
  (Variables|Default|SetHealth (Math|Float|Clamp(Float) (- (Variables|Default|GetHealth) Damage) 0.0 (Variables|Default|GetMaxHealth)))
  (bind _asw_radial_health (Utilities|Casting|CastToW_RadialHealth (UserInterface|GetWidget (Variables|Default|GetRadialHealth))))
  (bind _output_get (Variables|/Game/Main/UserInterface/Health/W_RadialHealth.W_RadialHealth_C|SetHealth _asw_radial_health (Variables|Default|GetHealth)))
  (Variables|/Game/Main/UserInterface/Health/W_RadialHealth.W_RadialHealth_C|SetMaxHealth _asw_radial_health (Variables|Default|GetMaxHealth))
  (Math|Float|CompareFloat _output_get 0.0
    (:==
      _)
    (:<
      _))
  (Variables|Default|SetisDead true)
  (Physics|SetSimulatePhysics _mesh true)
  (Physics|AddImpulse _mesh "0.000000,0.000000,-600.000000" "None" false)
  (Collision|SetCollisionEnabled (Variables|Collision|GetCapsuleComponent) "NoCollision")
  (CallFunction|UpdateHighlight false))

(event EventTick
  (params (DeltaSeconds :type Float%20%28single-precision%29))
  (Utilities|FlowControl|Sequence
    (:then_0
      (if (Utilities|Array|IsNotEmpty (Collision|GetOverlappingActors "/Game/Main/Maps/LevelElements/Hazard/BP_SunRays.BP_SunRays_C" :!class /Script/Engine.Actor))
        (if (Variables|Default|GetisDead)
          (bind _tl_animation (Timeline|Timeline_0 Play)
            (:Update
              (Niagara|SetNiagaraVariable(Float) (Variables|Default|GetNS_Leak) "User_Animation" _tl_animation)
              (Rendering|Material|SetMaterial (Variables|Character|GetMesh) 0 "/Game/Main/Entities/Enemies/DissolveBurnVFX/M_SOL.M_SOL")
              (Rendering|Material|SetMaterial (Variables|Character|GetMesh) 1 "/Game/Main/Entities/Enemies/DissolveBurnVFX/M_SOL.M_SOL")
              (Rendering|Material|SetScalarParameterValueonMaterials (Variables|Character|GetMesh) "Animation" _tl_animation))
            (:Finished
              (Actor|DestroyActor))))
        (else
          (Timeline|Timeline_0 Stop))))
    (:then_1
      (Transformation|SetWorldRotation (Variables|Default|GetRadialHealth) (Math|Rotator|MakeRotator 0.0 9e+01 (- (.yaw (Transformation|GetWorldRotation (Variables|/Script/Engine.Actor|GetRootComponent (.CameraRef (CallFunction|GetPlayerRef))))) 1.8e+02)) false false))))

(event EventBeginPlay
  (Utilities|FlowControl|Sequence
    (:then_0
      (Variables|Default|SetCharacter%20Reference (.PlayerRef (CallFunction|GetPlayerRef))))
    (:then_1
      (bind _asw_radial_health (Utilities|Casting|CastToW_RadialHealth (UserInterface|GetWidget (Variables|Default|GetRadialHealth))))
      (Variables|/Game/Main/UserInterface/Health/W_RadialHealth.W_RadialHealth_C|SetHealth _asw_radial_health (Variables|Default|GetHealth))
      (Variables|/Game/Main/UserInterface/Health/W_RadialHealth.W_RadialHealth_C|SetMaxHealth _asw_radial_health (Variables|Default|GetMaxHealth)))))

(fn ConstructionScript)

(fn UpdateWalkSpeed
  (params (NewWalkSpeed :type Float%20%28double-precision%29))
  (Variables|/Script/Engine.CharacterMovementComponent|SetMaxWalkSpeed (Variables|Character|GetCharacterMovement) NewWalkSpeed))

(fn UpdateHighlight
  (params (HighlightState :type Boolean))
  (bind _mesh (Variables|Character|GetMesh))
  (if (Variables|Default|GetisDead)
    (Rendering|Material|SetOverlayMaterial _mesh 0 :!class /Script/Engine.MeshComponent :!label _label)
    (elif true
      (Rendering|Material|SetOverlayMaterial _mesh (Variables|Default|GetOverlayMaterial) :!class /Script/Engine.MeshComponent)
      (else
        (goto _label)))))

(fn EnemyRef
  (return self))