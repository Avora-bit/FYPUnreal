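; BP_Goal is the level goal actor that scores the objective and opens the LevelCompletion level when triggered.
; A GoalCol overlap or DebugSphere hit runs the same chain, without checking which actor triggered it.
; The chain casts player 0's character to IsometricOrbitCharacter, calls ObjectiveScore, then opens the level.
; It then sets Game and UI input, unpauses, and enables the mouse cursor, click and hover events.
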(event OnComponentBeginOverlap(GoalCol)
  (params (OverlappedComponent :type Primitive%20Component%20Object%20Reference) (OtherActor :type Actor%20Object%20Reference) (OtherComp :type Primitive%20Component%20Object%20Reference) (OtherBodyIndex :type Integer) (bFromSweep :type Boolean) (SweepResult :type Hit%20Result%20Structure%20%28by%20ref%29))
  (bind _returnvalue (Game|GetPlayerController 0))
  ;[1 1 1] Open Level
  (bind _asisometric_orbit_character (Utilities|Casting|CastToIsometricOrbitCharacter (Game|GetPlayerCharacter 0)))
  (Default|ObjectiveScore _asisometric_orbit_character)
  (Game|OpenLevel(byObjectReference) "/Game/Main/UserInterface/Menus/LevelCompletion/LevelCompletion.LevelCompletion")
  (Input|SetInputModeGameandUI _returnvalue 0 "DoNotLock" true false)
  (Game|SetGamePaused false)
  (Variables|/Script/Engine.PlayerController|SetbShowMouseCursor _returnvalue true)
  (Variables|/Script/Engine.PlayerController|SetbEnableClickEvents _returnvalue true)
  (Variables|/Script/Engine.PlayerController|SetbEnableMouseOverEvents _returnvalue true))

(event OnComponentHit(DebugSphere)
  (params (HitComponent :type Primitive%20Component%20Object%20Reference) (OtherActor :type Actor%20Object%20Reference) (OtherComp :type Primitive%20Component%20Object%20Reference) (NormalImpulse :type Vector :default "0, 0, 0") (Hit :type Hit%20Result%20Structure%20%28by%20ref%29))
  (bind _returnvalue (Game|GetPlayerController 0))
  ;[1 1 1] Open Level
  (bind _asisometric_orbit_character (Utilities|Casting|CastToIsometricOrbitCharacter (Game|GetPlayerCharacter 0)))
  (Default|ObjectiveScore _asisometric_orbit_character)
  (Game|OpenLevel(byObjectReference) "/Game/Main/UserInterface/Menus/LevelCompletion/LevelCompletion.LevelCompletion")
  (Input|SetInputModeGameandUI _returnvalue 0 "DoNotLock" true false)
  (Game|SetGamePaused false)
  (Variables|/Script/Engine.PlayerController|SetbShowMouseCursor _returnvalue true)
  (Variables|/Script/Engine.PlayerController|SetbEnableClickEvents _returnvalue true)
  (Variables|/Script/Engine.PlayerController|SetbEnableMouseOverEvents _returnvalue true))

(event EventBeginPlay)

(event Collision|EventActorBeginOverlap
  (params (OtherActor :type Actor%20Object%20Reference)))

(event EventTick
  (params (DeltaSeconds :type Float%20%28single-precision%29)))

(fn ConstructionScript)