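; BP_TestInvPickUP is a test interactable item pickup for the inventory.
; Its construction script applies the ModelToSwitch mesh to ItemModel.
; LookAt uses the ItemID row handle on BPItemDataComponent to look up the item's name and returns a "Pick up" prompt.
; Pickup prints a message and destroys the actor after a brief delay, with no inventory transfer here, and Interactwith is empty.
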(event EventBeginPlay)

(event Collision|EventActorBeginOverlap
  (params (OtherActor :type Actor%20Object%20Reference)))

(event EventTick
  (params (DeltaSeconds :type Float%20%28single-precision%29)))

(event EventPickup
  (Development|PrintString "Item has be picked up")
  (Utilities|FlowControl|Delay 0.1)
  (Actor|DestroyActor))

(event EventInteractwith)

(fn ConstructionScript
  (Components|StaticMesh|SetStaticMesh (Variables|Default|GetItemModel) (Variables|Default|GetModelToSwitch)))

(fn Lookat
  (bind _bp_itemdatacomponent (Variables|Default|GetBP_ItemDataComponent))
  (bind _itemid (Variables|/Game/Main/UserInterface/Inventory/Functions/BP_ItemDataComponent.BP_ItemDataComponent_C|GetItemID _bp_itemdatacomponent))
  (bind _returnvalue (Utilities|GetDataTableRow (.datatable _itemid) (.rowname _itemid))
    (:then
      (return (Utilities|Text|FormatText "Pick up {item}" (.Name (Utilities|Struct|BreakFItemStruct _returnvalue)))))))