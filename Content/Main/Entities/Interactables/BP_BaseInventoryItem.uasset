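; Base actor for world items that the player can store in an inventory and drop again.
; Sphere overlap toggles an overlay-material highlight and an interaction widget, which Tick can keep above the mesh.
; StoreThisItem adds the item to the player's rock slot or general inventory, then hides it and disables physics and collision.
; DropThisItem moves the same actor to a location, unhides it and restores collision, but not physics simulation.
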(event OnComponentBeginOverlap(SphereCollider)
  (params (OverlappedComponent :type Primitive%20Component%20Object%20Reference) (OtherActor :type Actor%20Object%20Reference) (OtherComp :type Primitive%20Component%20Object%20Reference) (OtherBodyIndex :type Integer) (bFromSweep :type Boolean) (SweepResult :type Hit%20Result%20Structure%20%28by%20ref%29))
  (CallFunction|UpdateHighlight true)
  (CallFunction|UpdateInteractionPopup true false false false false false))

(event OnComponentEndOverlap(SphereCollider)
  (params (OverlappedComponent :type Primitive%20Component%20Object%20Reference) (OtherActor :type Actor%20Object%20Reference) (OtherComp :type Primitive%20Component%20Object%20Reference) (OtherBodyIndex :type Integer))
  (CallFunction|UpdateHighlight false)
  (CallFunction|UpdateInteractionPopup false false false false false false))

(event EventBeginPlay
  (bind _self self)
  (Variables|Default|SetPlayerRef (.PlayerRef (CallFunction|GetPlayerRef)))
  (Variables|Default|SetItemStructure (Utilities|Struct|MakeS_InventoryItem _self (Utilities|GetClass _self) (Variables|Default|GetItemName) (Variables|Default|GetItemImage)))
  (Rendering|SetVisibility (Variables|Default|GetInteractPopUp) false false))

(event EventTick
  (params (DeltaSeconds :type Float%20%28single-precision%29))
  (Utilities|FlowControl|Sequence
    (:then_0
      (if (Variables|Default|GetDisplayPopup)
        (Transformation|SetWorldLocation (Variables|Default|GetInteractPopUp) (+ (Transformation|GetWorldLocation (Variables|Default|GetStaticMesh)) "0.000000,0.000000,50.000000") false false)))))

(fn ConstructionScript)

(fn StoreThisItem
  (params (PreAllocatedSlot :type Boolean))
  (bind _self self)
  (bind _playerref (Variables|Default|GetPlayerRef))
  (if PreAllocatedSlot
    (bind _success (Default|AddRocktoInventory _playerref _self))
    (if _success
      (Physics|SetSimulatePhysics (Variables|Default|GetStaticMesh) false :!label _label)
      (Collision|SetCollisionEnabled (Variables|Default|GetSphere%20Collider) "NoCollision")
      (Rendering|SetActorHiddenInGame true)
      (else
        (Development|PrintString "Rock Full")))
    (else
      (bind _success_2 (Default|AddItemtoInventory _playerref _self))
      (if _success_2
        (goto _label)
        (else
          (Development|PrintString "Inventory Full"))))))

(fn DropThisItem
  (params (Drop%20Location :type Vector))
  (Transformation|SetActorLocation Drop%20Location false false)
  (Collision|SetCollisionEnabled (Variables|Default|GetSphere%20Collider) "QueryAndPhysics")
  (Rendering|SetActorHiddenInGame false))

(fn UpdateInteractionPopup
  (params (Visibility :type Boolean) (Interact :type Boolean) (Pickup :type Boolean) (Eat :type Boolean) (Unlock :type Boolean) (Open/Close :type Boolean))
  (bind _interactpopup (Variables|Default|GetInteractPopUp))
  (bind _asw_interactions (Utilities|Casting|CastToW_Interactions (UserInterface|GetWidget _interactpopup)))
  (Rendering|SetVisibility _interactpopup Visibility false)
  (Variables|/Game/Main/UserInterface/Interactables/W_Interactions.W_Interactions_C|SetIsInteract _asw_interactions Interact)
  (Variables|/Game/Main/UserInterface/Interactables/W_Interactions.W_Interactions_C|SetIsPickup _asw_interactions Pickup)
  (Variables|/Game/Main/UserInterface/Interactables/W_Interactions.W_Interactions_C|SetIsEat _asw_interactions Eat)
  (Variables|/Game/Main/UserInterface/Interactables/W_Interactions.W_Interactions_C|SetIsUnlock _asw_interactions Unlock)
  (Variables|/Game/Main/UserInterface/Interactables/W_Interactions.W_Interactions_C|SetIsOpen _asw_interactions Open/Close)
  (Default|UpdateData _asw_interactions))

(fn UpdateHighlight
  (params (Visibility :type Boolean))
  (bind _staticmesh (Variables|Default|GetStaticMesh))
  (if Visibility
    (Rendering|Material|SetOverlayMaterial _staticmesh (Variables|Default|GetOverlayMaterial) :!class /Script/Engine.MeshComponent)
    (else
      (Rendering|Material|SetOverlayMaterial _staticmesh 0 :!class /Script/Engine.MeshComponent))))