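; BP_Revolver is an interactable revolver item that can be picked up through interface events.
; On interact, it looks up its row in the data table via ACItemDataComponent, then plays a sound at its location and calls AddItem.
; On use, it turns off the sphere collider's overlap events and restores them after a timed delay.
; Debug prints and a StoreThisItem call remain unconnected.
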(event EventBPIInteract
  (bind _ac_itemdatacomponent (Variables|Default|GetAC_ItemDataComponent))
  (bind _itemid (Variables|/Game/Main/UserInterface/Inventory/AC_ItemDataComponent.AC_ItemDataComponent_C|GetItemID _ac_itemdatacomponent))
  (bind _returnvalue (Utilities|GetDataTableRow (.datatable _itemid) (.rowname _itemid))
    (:then
      (Audio|SpawnSoundatLocation (Variables|Default|GetInteractSound) (Transformation|GetActorLocation) "0, 0, 0" 1.0 1.0 0.0 0 0)
      (CallFunction|AddItem (Variables|Default|GetItemStructure)))))

(event EventBPIUse
  (bind _sphere_collider (Variables|Default|GetSphere%20Collider))
  (Variables|/Script/Engine.PrimitiveComponent|SetbGenerateOverlapEvents _sphere_collider false)
  (Utilities|FlowControl|Delay (Variables|Default|GetTimer))
  (Variables|/Script/Engine.PrimitiveComponent|SetbGenerateOverlapEvents _sphere_collider true))

(fn ConstructionScript)