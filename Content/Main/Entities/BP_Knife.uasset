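; BP_Knife is a knife item the player can pick up and use.
; Interacting looks up its row in the item data table via the item data component, plays a pickup sound, prints the item name and stores it as an item.
; Using the knife calls WeaponFire1 to perform its attack.
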(event EventBPIInteract
  (bind _ac_itemdatacomponent (Variables|Default|GetAC_ItemDataComponent))
  (bind _itemid (Variables|/Game/Main/UserInterface/Inventory/AC_ItemDataComponent.AC_ItemDataComponent_C|GetItemID _ac_itemdatacomponent))
  (bind _returnvalue (Utilities|GetDataTableRow (.datatable _itemid) (.rowname _itemid))
    (:then
      (Audio|SpawnSoundatLocation (Variables|Default|GetInteractSound) (Transformation|GetActorLocation) "0, 0, 0" 1.0 1.0 0.0 0 0)
      (Development|PrintText (Utilities|Text|FormatText "Picked up: {item}" (.Name (Utilities|Struct|BreakS_InventoryItem _returnvalue))))
      (CallFunction|StoreThisItem false (Variables|Default|GetItemStruct)))))

(event EventBPIUse
  (CallFunction|WeaponFire1))

(fn ConstructionScript)