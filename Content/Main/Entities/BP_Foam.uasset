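; BP_Foam is a foam actor that puts out fires it touches.
; When any valid actor begins overlapping it, it tells every BP_Fire inside its Capsule to dissipate.
; When an actor stops overlapping, it calls stop-dissipating on the fires still inside the Capsule, rather than on the actor that left.
; Both events print debug strings, and the construction script is empty.
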(event Collision|EventActorBeginOverlap
  (params (OtherActor :type Actor%20Object%20Reference))
  (Utilities|IsValid OtherActor
    (:Is%20Valid
      (for _array_element (Collision|GetOverlappingActors (Variables|Default|GetCapsule) "/Game/Main/Entities/BaseClasses/BP_Fire.BP_Fire_C" :!class /Script/Engine.PrimitiveComponent)
        (bind _asbp_fire (Utilities|Casting|CastToBP_Fire _array_element))
        (Default|DissapateFire _asbp_fire)
        (Development|PrintString "Putting Out Fire")))))

(event Collision|EventActorEndOverlap
  (params (OtherActor :type Actor%20Object%20Reference))
  (Utilities|IsValid OtherActor
    (:Is%20Valid
      (for _array_element (Collision|GetOverlappingActors (Variables|Default|GetCapsule) "/Game/Main/Entities/BaseClasses/BP_Fire.BP_Fire_C" :!class /Script/Engine.PrimitiveComponent)
        (bind _asbp_fire (Utilities|Casting|CastToBP_Fire _array_element))
        (Default|StopDissapting _asbp_fire)
        (Development|PrintString "stop burning")))))

(fn ConstructionScript)