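; Test sword NPC that chases players it sees or hears, leashed to its spawn point, with Attack still an empty stub.
; PawnSensing starts AI MoveTo and a retriggerable delay clears the sensed flag.
; Leaving the chase radius or losing the player sends it back to spawn, refilling health as the move starts.
; ChangeHealth caps healing, launches it upward on damage and destroys it at zero, but its EventGraph call is unwired.
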(event OnSeePawn(PawnSensing)
  (params (Pawn :type Pawn%20Object%20Reference))
  ;[1 1 1] Chase Player
  (bind _asbp_third_person_character (Utilities|Casting|CastToBP_ThirdPersonCharacter Pawn))
  (Utilities|FlowControl|Sequence
    (:then_0
      (Variables|Default|SetcanSensePlayer true)
      (AI|AIMoveTo self "0, 0, 0" _asbp_third_person_character 5.0 false
        (:OnSuccess
          (CallFunction|Attack)
          (if (Variables|Default|GetcanSensePlayer) :!label _label
            (Math|Float|CompareFloat (Variables|Default|GetChaseRadius) (Math|Vector|Distance(Vector) (Variables|Default|GetSpawn%20Location) (Transformation|GetActorLocation))
              (:==
                _)
              (:<
                _))
            (CallFunction|ReturntoSpawnpoint :!label _label_2)
            (Utilities|FlowControl|Delay 2.0)
            (goto _label)
            (else
              (Utilities|FlowControl|Delay (Variables|Default|GetChaseToIdleTimer))
              (if (not (Variables|Default|GetcanSensePlayer)) ; if cannot see player after a while go patrol
                (goto _label_2)))))))
    (:then_1
      (Utilities|FlowControl|RetriggerableDelay (Variables|Default|GetChaseToIdleTimer))
      (Variables|Default|SetcanSensePlayer false))))

(event OnHearNoise(PawnSensing)
  (params (Instigator :type Pawn%20Object%20Reference) (Location :type Vector%20%28by%20ref%29 :default "0, 0, 0") (Volume :type Float%20%28single-precision%29))
  ;[1 1 1] Chase Player
  (bind _asbp_third_person_character (Utilities|Casting|CastToBP_ThirdPersonCharacter Instigator))
  (Utilities|FlowControl|Sequence
    (:then_0
      (Variables|Default|SetcanSensePlayer true)
      (AI|AIMoveTo self "0, 0, 0" _asbp_third_person_character 5.0 false
        (:OnSuccess
          (CallFunction|Attack)
          (if (Variables|Default|GetcanSensePlayer) :!label _label
            (Math|Float|CompareFloat (Variables|Default|GetChaseRadius) (Math|Vector|Distance(Vector) (Variables|Default|GetSpawn%20Location) (Transformation|GetActorLocation))
              (:==
                _)
              (:<
                _))
            (CallFunction|ReturntoSpawnpoint :!label _label_2)
            (Utilities|FlowControl|Delay 2.0)
            (goto _label)
            (else
              (Utilities|FlowControl|Delay (Variables|Default|GetChaseToIdleTimer))
              (if (not (Variables|Default|GetcanSensePlayer)) ; if cannot see player after a while go patrol
                (goto _label_2)))))))
    (:then_1
      (Utilities|FlowControl|RetriggerableDelay (Variables|Default|GetChaseToIdleTimer))
      (Variables|Default|SetcanSensePlayer false))))

(event Custom|Attack
  ;[1 1 1] Attack
)

(event Custom|Return%20to%20Spawnpoint
  ;[1 1 1] Return to Spawnpoint
  (AI|AIMoveTo self (Variables|Default|GetSpawn%20Location) 0 5.0 false
    (:then
      (Variables|Default|SetHealth (Variables|Default|GetmaxHealth)))))

(event EventTick
  (params (DeltaSeconds :type Float%20%28single-precision%29))
  ;[1 1 1] Health
)

(event EventBeginPlay
  (Variables|Default|SetHealth (Variables|Default|GetmaxHealth))
  (Variables|Default|SetSpawn%20Location (Transformation|GetActorLocation)) ; when spawned, set spawn pos
  (if (Variables|Default|GetcanSensePlayer) :!label _label
    (Math|Float|CompareFloat (Variables|Default|GetChaseRadius) (Math|Vector|Distance(Vector) (Variables|Default|GetSpawn%20Location) (Transformation|GetActorLocation))
      (:==
        _)
      (:<
        _))
    (CallFunction|ReturntoSpawnpoint :!label _label_2)
    (Utilities|FlowControl|Delay 2.0)
    (goto _label)
    (else
      (Utilities|FlowControl|Delay (Variables|Default|GetChaseToIdleTimer))
      (if (not (Variables|Default|GetcanSensePlayer)) ; if cannot see player after a while go patrol
        (goto _label_2)))))

(fn ConstructionScript)

(fn ChangeHealth
  (params (IntValue :type Integer))
  (bind _maxhealth (Variables|Default|GetmaxHealth))
  (Variables|Default|SetHealth (+ (Variables|Default|GetHealth) IntValue))
  (Math|Integer|CompareInt IntValue
    (:>
      (Math|Integer|CompareInt (Variables|Default|GetHealth) _maxhealth
        (:>
          (Variables|Default|SetHealth _maxhealth))))
    (:<
      (Math|Integer|CompareInt (Variables|Default|GetHealth)
        (:>
          (Character|LaunchCharacter (* IntValue IntValue (Math|Vector|VectorUp)) false false))
        (:==
          (Actor|DestroyActor :!label _label))
        (:<
          (goto _label))))))