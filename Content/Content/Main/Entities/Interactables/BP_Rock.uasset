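; BP_Rock is an interactable rock item that can be picked up, stored and used.
; Interaction plays a sound at the rock's location, prints a pickup message and calls StoreThisItem.
; Using the item turns off overlap events on its SphereCollider, then restores them after a Timer delay.
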(event EventBPIUseItem
  (bind _sphere_collider (Variables|Default|GetSphere%20Collider))
  (Variables|/Script/Engine.PrimitiveComponent|SetbGenerateOverlapEvents _sphere_collider false)
  (Utilities|FlowControl|Delay (Variables|Default|GetTimer))
  (Variables|/Script/Engine.PrimitiveComponent|SetbGenerateOverlapEvents _sphere_collider true))

(event EventBPIInteraction
  (params (ChacterRef :type Isometric%20Orbit%20Character%20Object%20Reference))
  (Audio|SpawnSoundatLocation (Variables|Default|GetInteractSound) (Transformation|GetActorLocation) "0, 0, 0" 1.0 1.0 0.0 0 0)
  (Development|PrintString "Rock Picked up")
  (CallFunction|StoreThisItem true))

(fn ConstructionScript)