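; Enemy NPC that patrols around its spawn point and chases the third-person player on sight, with an empty Attack stub.
; A delayed BeginPlay loop compares spawn distance against chase or roam radius to roam or return home, restoring health.
; PawnSensing sight and hearing set the sensed flag, cleared by retriggerable delays; only sight starts movement.
; ChangeHealth clamps healing, launches upward on damage and destroys at zero, but the event graph never runs it.
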(event OnSeePawn(PawnSensing)
  (params (Pawn :type Pawn%20Object%20Reference))
  (bind _returnvalue (Transformation|GetActorLocation))
  (bind _spawn_location (Variables|Default|GetSpawn%20Location))
  (bind _returnvalue_2 (Math|Vector|Distance(Vector) _spawn_location _returnvalue))
  ;[1 1 1] Chase Player
  (bind _asbp_third_person_character (Utilities|Casting|CastToBP_ThirdPersonCharacter Pawn))
  (Utilities|FlowControl|Sequence
    (:then_0
      (Variables|Default|SetcanSensePlayer true)
      (AI|AIMoveTo (AI|GetAIController self) "0, 0, 0" _asbp_third_person_character -1.0 "Default" "Default" true true
        (:then
          (CallFunction|Attack)
          (if (Variables|Default|GetcanSensePlayer) :!label _label
            (Math|Float|CompareFloat (Variables|Default|GetChaseRadius) _returnvalue_2
              (:==
                _)
              (:<
                _))
            (CallFunction|ReturntoSpawnpoint :!label _label_2)
            (Utilities|FlowControl|Delay 2.0 :!label _label_3)
            (goto _label)
            (else
              (Utilities|FlowControl|Delay (Variables|Default|GetChaseToIdleTimer))
              (if (not (Variables|Default|GetcanSensePlayer)) ; if cannot see player after a while go patrol
                (Math|Float|CompareFloat (Variables|Default|GetRoamRadius) _returnvalue_2
                  (:>
                    (CallFunction|RandomRoam)
                    (goto _label_3))
                  (:==
                    (goto _label_2))
                  (:<
                    (goto _label_2)))))))))
    (:then_1
      (Utilities|FlowControl|RetriggerableDelay (Variables|Default|GetChaseToIdleTimer))
      (Variables|Default|SetcanSensePlayer false))))

(event OnHearNoise(PawnSensing)
  (params (Instigator :type Pawn%20Object%20Reference) (Location :type Vector%20%28by%20ref%29 :default "0, 0, 0") (Volume :type Float%20%28single-precision%29))
  ;[1 1 1] Chase Player
  (bind _asbp_third_person_character (Utilities|Casting|CastToBP_ThirdPersonCharacter Instigator))
  (Utilities|FlowControl|Sequence
    (:then_0
      (Variables|Default|SetcanSensePlayer true))
    (:then_1
      (Utilities|FlowControl|RetriggerableDelay (Variables|Default|GetChaseToIdleTimer))
      (Variables|Default|SetcanSensePlayer false))))

(event Custom|RandomRoam
  ;[1 1 1] Patrol Around Spawn
  (bind _output_get (Variables|Default|SetRandom%20Location (.RandomLocation (AI|Navigation|GetRandomReachablePointinRadius (Variables|Default|GetSpawn%20Location) (Variables|Default|GetRoamRadius) 0 0))))
  (AI|AIMoveTo self _output_get 0 5.0 false))

(event Custom|Attack
  ;[1 1 1] Attack
)

(event Custom|Return%20to%20Spawnpoint
  ;[1 1 1] Return to Spawnpoint
  (AI|AIMoveTo self (Variables|Default|GetSpawn%20Location) 0 5.0 false
    (:then
      (Variables|Default|SetHealth (Variables|Default|GetmaxHealth)))))

(event EventTick
  (params (DeltaSeconds :type Float%20%28single-precision%29))
  ;[1 1 1] Health
)

(event EventBeginPlay
  (Variables|Default|SetHealth (Variables|Default|GetmaxHealth))
  (Variables|Default|SetSpawn%20Location (Transformation|GetActorLocation)) ; when spawned, set spawn pos
  (if (Variables|Default|GetcanSensePlayer) :!label _label
    (Math|Float|CompareFloat (Variables|Default|GetChaseRadius) (Math|Vector|Distance(Vector) (Variables|Default|GetSpawn%20Location) (Transformation|GetActorLocation))
      (:==
        _)
      (:<
        _))
    (CallFunction|ReturntoSpawnpoint :!label _label_2)
    (Utilities|FlowControl|Delay 2.0 :!label _label_3)
    (goto _label)
    (else
      (Utilities|FlowControl|Delay (Variables|Default|GetChaseToIdleTimer))
      (if (not (Variables|Default|GetcanSensePlayer)) ; if cannot see player after a while go patrol
        (Math|Float|CompareFloat (Variables|Default|GetRoamRadius) (Math|Vector|Distance(Vector) (Variables|Default|GetSpawn%20Location) (Transformation|GetActorLocation))
          (:>
            (CallFunction|RandomRoam)
            (goto _label_3))
          (:==
            (goto _label_2))
          (:<
            (goto _label_2)))))))

(fn ConstructionScript)

(fn ChangeHealth
  (params (IntValue :type Integer))
  (bind _maxhealth (Variables|Default|GetmaxHealth))
  (Variables|Default|SetHealth (+ (Variables|Default|GetHealth) IntValue))
  (Math|Integer|CompareInt IntValue
    (:>
      (Math|Integer|CompareInt (Variables|Default|GetHealth) _maxhealth
        (:>
          (Variables|Default|SetHealth _maxhealth))))
    (:<
      (Math|Integer|CompareInt (Variables|Default|GetHealth)
        (:>
          (Character|LaunchCharacter (* IntValue IntValue (Math|Vector|VectorUp)) false false))
        (:==
          (Actor|DestroyActor :!label _label))
        (:<
          (goto _label))))))