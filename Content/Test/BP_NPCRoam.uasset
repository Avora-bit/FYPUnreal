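; Test NPC that roams around its spawn point, chases the third-person player character and returns home when it strays too far.
; A delay-driven loop compares distance from spawn against chase and roam radii, choosing a random reachable destination or a return to spawn.
; PawnSensing sight and noise events share the AI MoveTo chase, with a retriggerable delay clearing the player-seen flag.
; The Attack event is an empty stub.
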(event OnSeePawn(PawnSensing)
  (params (Pawn :type Pawn%20Object%20Reference))
  (bind _returnvalue (Transformation|GetActorLocation))
  (bind _spawn_location (Variables|Default|GetSpawn%20Location))
  (bind _returnvalue_2 (Math|Vector|Distance(Vector) _spawn_location _returnvalue))
  ;[1 1 1] Chase Player
  (bind _asbp_third_person_character (Utilities|Casting|CastToBP_ThirdPersonCharacter Pawn))
  (Utilities|FlowControl|Sequence
    (:then_0
      (Variables|Default|SetcanSeePlayer true)
      (AI|AIMoveTo self "0, 0, 0" _asbp_third_person_character 5.0 false
        (:OnSuccess
          _)
        (:OnFail
          _))
      (if (Variables|Default|GetcanSeePlayer) :!label _label
        (Math|Float|CompareFloat (Variables|Default|GetChaseRadius) _returnvalue_2
          (:==
            _)
          (:<
            _))
        (CallFunction|ReturntoSpawnpoint :!label _label_2)
        (Utilities|FlowControl|Delay 2.0 :!label _label_3)
        (goto _label)
        (else
          (Utilities|FlowControl|Delay (Variables|Default|GetChaseToIdleTimer))
          (if (not (Variables|Default|GetcanSeePlayer)) ; if cannot see player after a while go patrol
            (Math|Float|CompareFloat (Variables|Default|GetRoamRadius) _returnvalue_2
              (:>
                (CallFunction|MoveNPC)
                (goto _label_3))
              (:==
                (goto _label_2))
              (:<
                (goto _label_2)))))))
    (:then_1
      (Utilities|FlowControl|RetriggerableDelay (Variables|Default|GetChaseToIdleTimer))
      (Variables|Default|SetcanSeePlayer false))))

(event OnHearNoise(PawnSensing)
  (params (Instigator :type Pawn%20Object%20Reference) (Location :type Vector%20%28by%20ref%29 :default "0, 0, 0") (Volume :type Float%20%28single-precision%29))
  (bind _returnvalue (Transformation|GetActorLocation))
  (bind _spawn_location (Variables|Default|GetSpawn%20Location))
  (bind _returnvalue_2 (Math|Vector|Distance(Vector) _spawn_location _returnvalue))
  ;[1 1 1] Chase Player
  (bind _asbp_third_person_character (Utilities|Casting|CastToBP_ThirdPersonCharacter (stale OnSeePawn(PawnSensing) Pawn)))
  (Utilities|FlowControl|Sequence
    (:then_0
      (Variables|Default|SetcanSeePlayer true)
      (AI|AIMoveTo self "0, 0, 0" _asbp_third_person_character 5.0 false
        (:OnSuccess
          _)
        (:OnFail
          _))
      (if (Variables|Default|GetcanSeePlayer) :!label _label
        (Math|Float|CompareFloat (Variables|Default|GetChaseRadius) _returnvalue_2
          (:==
            _)
          (:<
            _))
        (CallFunction|ReturntoSpawnpoint :!label _label_2)
        (Utilities|FlowControl|Delay 2.0 :!label _label_3)
        (goto _label)
        (else
          (Utilities|FlowControl|Delay (Variables|Default|GetChaseToIdleTimer))
          (if (not (Variables|Default|GetcanSeePlayer)) ; if cannot see player after a while go patrol
            (Math|Float|CompareFloat (Variables|Default|GetRoamRadius) _returnvalue_2
              (:>
                (CallFunction|MoveNPC)
                (goto _label_3))
              (:==
                (goto _label_2))
              (:<
                (goto _label_2)))))))
    (:then_1
      (Utilities|FlowControl|RetriggerableDelay (Variables|Default|GetChaseToIdleTimer))
      (Variables|Default|SetcanSeePlayer false))))

(event Custom|MoveNPC
  ;[1 1 1] Patrol Around Spawn
  (bind _output_get (Variables|Default|SetRandom%20Location (.RandomLocation (AI|Navigation|GetRandomReachablePointinRadius (Variables|Default|GetSpawn%20Location) (Variables|Default|GetRoamRadius) 0 0))))
  (AI|AIMoveTo self _output_get 0 5.0 false))

(event Custom|Attack
  ;[1 1 1] Attack
)

(event Custom|Return%20to%20Spawnpoint
  ;[1 1 1] Return to Spawnpoint
  (AI|AIMoveTo self (Variables|Default|GetSpawn%20Location) 0 5.0 false))

(event EventBeginPlay
  (Variables|Default|SetSpawn%20Location (Transformation|GetActorLocation)) ; when spawned, set spawn pos
  (if (Variables|Default|GetcanSeePlayer) :!label _label
    (Math|Float|CompareFloat (Variables|Default|GetChaseRadius) (Math|Vector|Distance(Vector) (Variables|Default|GetSpawn%20Location) (Transformation|GetActorLocation))
      (:==
        _)
      (:<
        _))
    (CallFunction|ReturntoSpawnpoint :!label _label_2)
    (Utilities|FlowControl|Delay 2.0 :!label _label_3)
    (goto _label)
    (else
      (Utilities|FlowControl|Delay (Variables|Default|GetChaseToIdleTimer))
      (if (not (Variables|Default|GetcanSeePlayer)) ; if cannot see player after a while go patrol
        (Math|Float|CompareFloat (Variables|Default|GetRoamRadius) (Math|Vector|Distance(Vector) (Variables|Default|GetSpawn%20Location) (Transformation|GetActorLocation))
          (:>
            (CallFunction|MoveNPC)
            (goto _label_3))
          (:==
            (goto _label_2))
          (:<
            (goto _label_2)))))))

(fn ConstructionScript)